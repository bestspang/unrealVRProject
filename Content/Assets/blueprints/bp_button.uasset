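; A VR push button Blueprint that animates its mesh when a motion controller touches it.
; An overlap with a BP_MotionController's GrabSphere plays a timeline that lerps the button mesh's relative scale between starting and ending values.
; Ending the overlap, by any component, reverses the timeline to restore the scale.
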(event `self.button_mesh.OnComponentBeginOverlap`
  (params (OverlappedComponent :type "PrimitiveComponent Object Reference") (OtherActor :type "Actor Object Reference") (OtherComp :type "PrimitiveComponent Object Reference") (OtherBodyIndex :type Integer) (bFromSweep :type Boolean) (SweepResult :type "HitResult Structure (by ref)"))
  (bind _asbp_motion_controller (cast `/Game/Assets/player/BP_MotionController` OtherActor))
  (if (== (`/Game/Assets/player/BP_MotionController.grabSphere` _asbp_motion_controller) OtherComp)
    (bind (_direction _alpha) (`Timeline|animation` :!label _label)
      (:`Update`
        (`SceneComponent.SetRelativeScale3D` (`self.button_mesh`) (`KismetMathLibrary.VLerp` (`self.startingScale`) (`self.endingScale`) _alpha))))))

(event `self.button_mesh.OnComponentEndOverlap`
  (params (OverlappedComponent :type "PrimitiveComponent Object Reference") (OtherActor :type "Actor Object Reference") (OtherComp :type "PrimitiveComponent Object Reference") (OtherBodyIndex :type Integer))
  (goto _label :!via `Reverse`))

(fn `UserConstructionScript`)