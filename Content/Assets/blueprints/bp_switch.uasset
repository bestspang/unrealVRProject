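; VR light switch Blueprint that toggles every bp_light tagged for a room when a motion controller's GrabSphere enters its Box.
; GetLight applies the IsOn state to the tagged lights at BeginPlay and on each toggle.
; An IsOverlap latch prevents retriggering; Tick, rather than the empty end-overlap event, clears it.
; The construction script derives RoomTag from RoomEnum, except one entry that keeps a manual tag and warns when None.
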(event `self.ReceiveTick`
  (params (DeltaSeconds :type "Float (single-precision)"))
  (bind _box (`self.Box`))
  (bind _overlappingactors (`PrimitiveComponent.GetOverlappingActors` _box "/Game/Assets/player/BP_MotionController.BP_MotionController_C"))
  (if (`KismetArrayLibrary.Array_IsValidIndex` _overlappingactors)
    (bind _asbp_motion_controller (cast `/Game/Assets/player/BP_MotionController` (`|GetArrayItem` _overlappingactors)))
    (if (not (`PrimitiveComponent.IsOverlappingComponent` _box (`/Game/Assets/player/BP_MotionController.grabSphere` _asbp_motion_controller)))
      (set `self.isOverlap` false))
    (else
      (set `self.isOverlap` false))))

(event `self.ReceiveBeginPlay`
  (`self.getLight` (`self.roomTag`) (`self.isOn`)))

(event `self.Box.OnComponentBeginOverlap`
  (params (OverlappedComponent :type "PrimitiveComponent Object Reference") (OtherActor :type "Actor Object Reference") (OtherComp :type "PrimitiveComponent Object Reference") (OtherBodyIndex :type Integer) (bFromSweep :type Boolean) (SweepResult :type "HitResult Structure (by ref)"))
  (if (not (`self.isOverlap`))
    (bind _asbp_motion_controller (cast `/Game/Assets/player/BP_MotionController` OtherActor))
    (if (== (`/Game/Assets/player/BP_MotionController.grabSphere` _asbp_motion_controller) OtherComp)
      (if (`self.isOn`)
        (set `self.isOn` false)
        (else
          (set `self.isOn` true)))
      (set `self.isOverlap` true)
      (`self.getLight` (`self.roomTag`) (`self.isOn`)))))

(event `self.Box.OnComponentEndOverlap`
  (params (OverlappedComponent :type "PrimitiveComponent Object Reference") (OtherActor :type "Actor Object Reference") (OtherComp :type "PrimitiveComponent Object Reference") (OtherBodyIndex :type Integer)))

(fn `getLight`
  (params (roomTag :type Name) (isOn :type Boolean))
  (bind _outactors (`GameplayStatics.GetAllActorsWithTag` roomTag))
  (if isOn
    (for _array_element _outactors
      (bind _asbp_light (cast `/Game/Assets/blueprints/bp_light` _array_element))
      (`/Game/Assets/blueprints/bp_light.TurnOn` _asbp_light))
    (else
      (for _array_element_2 _outactors
        (bind _asbp_light_2 (cast `/Game/Assets/blueprints/bp_light` _array_element_2))
        (`/Game/Assets/blueprints/bp_light.TurnOff` _asbp_light_2)))))

(fn `UserConstructionScript`
  (bind _roomenum (`self.roomEnum`))
  (bind _roomtag (`self.roomTag`))
  (if (`|EnumEquality` _roomenum "NewEnumerator3")
    (if (!= _roomtag "None")
      (set `self.roomTag` _roomtag)
      (else
        (`KismetSystemLibrary.PrintString` "NO TAG!" true true (struct :`R` 1.0 :`B` 0.079394 :`A` 1.0))))
    (else
      (set `self.roomTag` (`|GetEnumeratorName` _roomenum)))))