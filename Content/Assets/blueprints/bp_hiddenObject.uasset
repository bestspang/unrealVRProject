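; Hidden object actor for a VR game that can be grabbed, dropped and popped like a balloon, with fake ones given a random color.
; On BeginPlay it binds to the pop event of BP_MyVRPawnOLD, which triggers a scale timeline, then confetti, sound and destruction.
; Pickup and drop toggle physics, collision and hand attachment, and set the grab flag on BP_MyVRPawnTest, a different pawn class.
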(event `playAnimation`
  ;[0.1349 1 0.07292] animation
  (bind (_direction _alpha) (`Timeline|animation`)
    (:`Update`
      (`SceneComponent.SetRelativeScale3D` (`self.hiddenMesh`) (`KismetMathLibrary.VLerp` (`self.startingScale`) (`self.endingScale`) _alpha)))))

(event `self.ReceiveBeginPlay`
  (bind _colorarray (`self.colorArray`))
  ;[1 1 1] setup
  (`|ExecutionSequence`
    (:`then_0`
      ;[1 1 1] set colors array
      (set `self.colorArray` (`|MakeArray` (0.0 0.0 0.0) (0.0 1.0 0.0) (0.0 0.0 1.0) (1.0 1.0 0.0) (0.0 1.0 1.0) (1.0 0.0 1.0) (1.0 1.0 1.0) :!type "Vector Structure"))
      (set `self.startingScale` (`SceneComponent.K2_GetComponentScale` (`self.hiddenMesh`))))
    (:`then_1`
      ;[1 0.301 0.01818] apply color
      (if (`self.isFake`)
        (`MeshComponent.SetVectorParameterValueOnMaterials` (`self.hiddenMesh`) "colorBase" (`|GetArrayItem` _colorarray (`KismetMathLibrary.RandomIntegerInRange` 0 (- (`KismetArrayLibrary.Array_Length` _colorarray) 1))))))
    (:`then_2`
      ;[1 1 1] bind event prepare for pop
      (bind _outactors (`GameplayStatics.GetAllActorsOfClass` "/Game/Assets/player/BP_MyVRPawnOLD.BP_MyVRPawnOLD_C"))
      (bind _output_get (set `self.myVRPawn` (`|GetArrayItem` _outactors)))
      (add `/Game/Assets/player/BP_MyVRPawnOLD.popHiddenObjects` _output_get (delegate `popped`)))))

(event `popped`
  (bind _returnvalue (`SceneComponent.K2_GetComponentLocation` (`self.hiddenMesh`)))
  ;[1 0.4519 0.07239] destroy balloon
  (`self.playAnimation`)
  (if true
    ;;[1 0.02277 0.6074] add sound and Particles
    (`KismetSystemLibrary.Delay` 0.1))
  (`GameplayStatics.SpawnEmitterAtLocation` "/Game/Assets/alternative_resources/p_confetti.p_confetti" _returnvalue)
  (`GameplayStatics.PlaySoundAtLocation` "/Game/Assets/audio/a_balloonPop_Cue.a_balloonPop_Cue" _returnvalue)
  (`self.K2_DestroyActor`))

(event `/Game/Assets/blueprints/bpi_grabbingInterface.pickUp`
  (params (ActorToAttachTo :type "SceneComponent Object Reference"))
  (bind _hiddenmesh (`self.hiddenMesh`))
  ;[0.2499 1 0.3458] Pickup and Drop
  (`PrimitiveComponent.SetSimulatePhysics` _hiddenmesh false)
  (`SceneComponent.K2_AttachToComponent` (`self.K2_GetRootComponent`) ActorToAttachTo "hand_LSocket" "KeepWorld" "KeepWorld" "KeepWorld" false)
  (bind _asbp_my_vrpawn_test (cast `/Game/Assets/player/BP_MyVRPawnTest` (`GameplayStatics.GetPlayerPawn` 0)))
  (set `/Game/Assets/player/BP_MyVRPawnTest.isGrab` true _asbp_my_vrpawn_test)
  (`PrimitiveComponent.SetCollisionEnabled` _hiddenmesh "PhysicsOnly"))

(event `/Game/Assets/blueprints/bpi_grabbingInterface.dropOff`
  (bind _hiddenmesh (`self.hiddenMesh`))
  ;[0.2499 1 0.3458] Pickup and Drop
  (`PrimitiveComponent.SetSimulatePhysics` _hiddenmesh true)
  (`SceneComponent.K2_DetachFromComponent` _hiddenmesh "KeepWorld" "KeepWorld" "KeepWorld" false)
  (bind _asbp_my_vrpawn_test (cast `/Game/Assets/player/BP_MyVRPawnTest` (`GameplayStatics.GetPlayerPawn` 0)))
  (set `/Game/Assets/player/BP_MyVRPawnTest.isGrab` false _asbp_my_vrpawn_test)
  (`PrimitiveComponent.SetCollisionEnabled` _hiddenmesh "QueryAndPhysics"))

(fn `UserConstructionScript`)