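; Physics object for a VR scene that can be highlighted, picked up, dropped and reset to its starting transform.
; On BeginPlay it stores its transform and binds a teleport-back event to the first BP_MyVRPawnTest's reset event.
; Pickup disables HiddenMesh physics and attaches the root to the given component; drop re-enables physics and detaches.
; Highlight and unhighlight toggle custom depth rendering on HiddenMesh.
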(event `self.ReceiveBeginPlay`
  (`|ExecutionSequence`
    (:`then_0`
      (set `self.initTransform` (`self.GetTransform`)))
    (:`then_1`
      (bind _outactors (`GameplayStatics.GetAllActorsOfClass` "/Game/Assets/player/BP_MyVRPawnTest.BP_MyVRPawnTest_C"))
      (bind _output_get (set `self.myVRPawn` (`|GetArrayItem` _outactors)))
      (add `/Game/Assets/player/BP_MyVRPawnTest.ResetObjects` _output_get (delegate `resetToInit`)))))

(event `resetToInit`
  (bind (_inittransform_location _inittransform_rotation) (`KismetMathLibrary.BreakTransform` (`self.initTransform`)))
  (`self.K2_TeleportTo` _inittransform_location _inittransform_rotation))

(event `/Game/Assets/blueprints/bpi_grabbingInterface.pickUp`
  (params (motionController :type "/Game/Assets/player/BP_MotionController Object Reference") (ActorToAttachTo :type "SceneComponent Object Reference"))
  ;[0.2499 1 0.3458] Pickup and Drop
  (`PrimitiveComponent.SetSimulatePhysics` (`self.hiddenMesh`) false)
  (`SceneComponent.K2_AttachToComponent` (`self.K2_GetRootComponent`) ActorToAttachTo "None" "KeepWorld" "KeepWorld" "KeepWorld" false))

(event `/Game/Assets/blueprints/bpi_grabbingInterface.dropOff`
  ;[0.2499 1 0.3458] Pickup and Drop
  (`PrimitiveComponent.SetSimulatePhysics` (`self.hiddenMesh`) true)
  (`self.K2_DetachFromActor` "KeepWorld" "KeepWorld" "KeepWorld"))

(fn `hightlight`
  (`PrimitiveComponent.SetRenderCustomDepth` (`self.hiddenMesh`) true))

(fn `unhightlight`
  (`PrimitiveComponent.SetRenderCustomDepth` (`self.hiddenMesh`) false))

(fn `UserConstructionScript`)