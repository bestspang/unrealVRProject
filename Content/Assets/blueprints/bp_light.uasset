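; bp_light is a light actor tagged by room, with functions that switch its Sphere's look between on and off.
; The construction script sets the actor tag from RoomEnum's name, except for one enumerator that uses the manual RoomTag and prints a red warning if it is "None".
; TurnOn and TurnOff swap the Sphere material and print debug strings; the event graph has no active logic.
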(event `self.ReceiveBeginPlay`)

(event `self.ReceiveTick`
  (params (DeltaSeconds :type "Float (single-precision)")))

(fn `TurnOff`
  (`PrimitiveComponent.SetMaterial` (`self.Sphere`) 0 "/Game/Assets/material/VRmat/M_BaseMaterial.M_BaseMaterial")
  (`KismetSystemLibrary.PrintString` "Hello"))

(fn `TurnOn`
  (`PrimitiveComponent.SetMaterial` (`self.Sphere`) 0 "/Game/Assets/material/Ballon_Mat_Inst.Ballon_Mat_Inst")
  (`KismetSystemLibrary.PrintString` "sdfsdf"))

(fn `UserConstructionScript`
  (bind _roomenum (`self.roomEnum`))
  (bind _roomtag (`self.roomTag`))
  (bind _returnvalue (`|GetEnumeratorName` _roomenum))
  (if (`|EnumEquality` _roomenum "NewEnumerator3")
    (if (!= _roomtag "None")
      (set `self.Tags` (`|MakeArray` _roomtag))
      (else
        (`KismetSystemLibrary.PrintString` "NO TAG!" true true (struct :`R` 1.0 :`B` 0.079394 :`A` 1.0))))
    (else
      (set `self.Tags` (`|MakeArray` _returnvalue))
      (set `self.roomTag` _returnvalue))))